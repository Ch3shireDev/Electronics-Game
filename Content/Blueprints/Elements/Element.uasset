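; Element Blueprint for a grabbable, movable object, with grab, drop and location-update hooks that are mostly stubs.
; Grabbing always returns HoldGlobal, and the default grab component is the root cast to a PrimitiveComponent.
; ManipulateElement moves non-socket components to the requested world location.
; For sockets with a starting position, it quantizes the location using a Y-axis delta but only prints it alongside that start, without moving the socket.
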(event Custom|Drop%20Element)

(event EventBeginPlay)

(fn ConstructionScript)

(fn GrabElement
  (params (Component :type Actor%20Component%20Object%20Reference))
  (return "VE_HoldGlobal"))

(fn UpdateElementLocation
  (params (Component :type Primitive%20Component%20Object%20Reference) (Location :type Transform)))

(fn GetDefaultGrabComponent
  (bind _asprimitive_component (Utilities|Casting|CastToPrimitiveComponent (VehicleSound|GetRootComponent))
    (:then
      _)
    (:CastFailed
      _))
  (return _asprimitive_component))

(fn ManipulateElement
  (params (NewWorldLocation :type Vector) (Component :type Primitive%20Component%20Object%20Reference))
  (bind (_startinglocation _returnvalue) (Class|CElement|GetSocketStartingPosition Component))
  (if (Class|CElement|IsSocket Component)
    (if _returnvalue
      (bind _returnvalue_2 (Class|CElement|QuantizePosition NewWorldLocation "0.000000,50.000000,0.000000"))
      (Development|PrintString (Utilities|String|Append (Utilities|String|ToString(Vector) _startinglocation) "   " (Utilities|String|ToString(Vector) _returnvalue_2))))
    (else
      (Class|CElement|SetElementPosition NewWorldLocation Component))))