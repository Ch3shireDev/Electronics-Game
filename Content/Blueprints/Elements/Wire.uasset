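; Wire element with two sockets that can be grabbed and moved, joined by spline mesh segments.
; GrabElement returns a local hold for either socket, a global hold for the root mesh and free otherwise.
; Location updates reposition sockets through WireLibrary, then destroy all spline mesh components and rebuild them.
; Tick has WireLibrary draw the points, while the logic that adds socket endpoints as points is unconnected.
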(event EventBeginPlay)

(event EventUpdateElementLocation
  (params (Component :type Primitive%20Component%20Object%20Reference) (Location :type Transform))
  (Class|WireLibrary|UpdateSocketPosition (Variables|Default|GetWireLibrary) Location self Component (Variables|Default|GetSocket%20A) (Variables|Default|GetSocket%20B))
  (CallFunction|RefreshWires))

(event EventTick
  (params (DeltaSeconds :type Float%20%28single-precision%29))
  (Class|WireLibrary|DrawPoints (Variables|Default|GetWireLibrary) self))

(fn ConstructionScript
  (|CallParentFunction))

(fn GrabElement
  (params (Component :type Actor%20Component%20Object%20Reference))
  (Utilities|SwitchonComponent Component (Variables|Default|GetSocket%20A) (Variables|Default|GetSocket%20B)
    (:Socket%20A
      _)
    (:Socket%20B
      _)
    (:Root%20Mesh
      (return "VE_HoldGlobal"))
    (:Else
      (return "VE_Free")))
  (return "VE_HoldLocal"))

(fn RefreshWires
  (for _array_element (Actor|GetComponentsByClass "/Script/Engine.SplineMeshComponent")
    (Components|DestroyComponent _array_element))
  (Class|WireLibrary|CreateWireParts (Variables|Default|GetWireLibrary) self (Variables|Default|GetScene1) "/Game/Meshes/WireMesh.WireMesh"))