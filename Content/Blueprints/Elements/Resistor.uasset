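; Resistor circuit element Blueprint built from Paper2D sprites that can be grabbed and held.
; Its construction script runs the parent's setup, then adds a socket at each of two secondary sprites; an older child-actor socket chain is left disconnected.
; The main sprite is the default grab component, and grabbing it returns a global hold, while grabbing any other component returns a local hold.
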(event EventBeginPlay)

(fn ConstructionScript
  (|CallParentFunction)
  (Class|CElement|AddSocket (Variables|Default|GetPaperSprite1))
  (Class|CElement|AddSocket (Variables|Default|GetPaperSprite2)))

(fn GetDefaultGrabComponent
  (return (Variables|Components|GetPaperSprite)))

(fn GrabElement
  (params (Component :type Actor%20Component%20Object%20Reference))
  (if (== Component (Variables|Components|GetPaperSprite))
    (return "VE_HoldGlobal")
    (else
      (return "VE_HoldLocal"))))