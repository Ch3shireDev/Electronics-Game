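; ElectronicsHUD manages mouse-driven placement of electronics Elements, creating the Menu widget and showing the cursor on BeginPlay.
; FindElementToGrab line-traces from the cursor when it is off the menu, grabbing the hit Element component and storing the hold type it returns.
; While held, Tick moves the element to the projected mouse position until DropElement frees it.
; SpawnElement spawns a given element class at that projected position.
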(event Custom|FindElementToGrab
  (bind _returnvalue (Game|GetPlayerController 0))
  (bind (_worldlocation _worlddirection) (Game|Player|ConvertMouseLocationToWorldSpace _returnvalue))
  (bind _mouse_over_menu (Default|IsMouseOverMenu (Variables|Default|GetMenuRef)))
  (if (not _mouse_over_menu)
    (bind (_outhit _returnvalue_2) (Collision|LineTraceByChannel _worldlocation (+ _worldlocation (* _worlddirection 2e+03)) "TraceTypeQuery1" false 0 "None"))
    (if _returnvalue_2
      (bind _aselement (Utilities|Casting|CastToElement (.HitActor (Collision|BreakHitResult _outhit))))
      (CallFunction|GrabElement _aselement (.HitComponent (Collision|BreakHitResult _outhit))))))

(event Custom|GrabElement
  (params (GrabElement :type Element%20Object%20Reference) (Component :type Primitive%20Component%20Object%20Reference))
  (bind _output_get (Variables|Default|SetElement%20Actor GrabElement))
  (bind _output_get_2 (Variables|Default|SetElement%20Component Component))
  (if (not (Variables|Default|GetbPlayerHoldsObject))
    (bind _hold_type (Default|GrabElement GrabElement _output_get_2))
    (Variables|Default|SetHoldType _hold_type)
    (Variables|Default|SetbPlayerHoldsObject true)
    (Development|PrintString "Grabbed!")))

(event Custom|MoveElement
  (if (not (Utilities|Enum|Equal(Enum) (Variables|Default|GetHoldType) "VE_Free"))
    (bind _outlocation (CallFunction|ProjectMouse))
    (Default|ManipulateElement (Variables|Default|GetElement%20Actor) _outlocation (Variables|Default|GetElement%20Component))))

(event Custom|DropElement
  (bind _element_actor (Variables|Default|GetElement%20Actor))
  (if (Math|Boolean|ANDBoolean (Variables|Default|GetbPlayerHoldsObject) (Utilities|IsValid _element_actor) (Utilities|IsValid (Variables|Default|GetElement%20Component)))
    (Default|DropElement _element_actor)
    (Variables|Default|SetHoldType "VE_Free")
    (Variables|Default|SetbPlayerHoldsObject false)))

(event EventBeginPlay
  (bind _returnvalue (Game|GetPlayerController 0))
  (bind _returnvalue_2 (UserInterface|CreateWidget "/Game/Widgets/Menu.Menu_C" _returnvalue))
  (UserInterface|Viewport|AddtoViewport _returnvalue_2 0)
  (Variables|Default|SetMenuRef _returnvalue_2)
  (Variables|/Script/Engine.PlayerController|SetbShowMouseCursor _returnvalue true)
  (Input|SetInputModeGameandUI _returnvalue (Variables|Default|GetMenuRef) "DoNotLock" false))

(event EventTick
  (params (DeltaSeconds :type Float%20%28single-precision%29))
  (CallFunction|MoveElement))

(fn ConstructionScript)

(fn SpawnElement
  (params (NewParam :type Element%20Class%20Reference))
  (bind _outlocation (CallFunction|ProjectMouse))
  (bind _returnvalue (Game|SpawnActorfromClass NewParam (Math|Transform|MakeTransform _outlocation) "AlwaysSpawn" 0 0))
  (Variables|Default|SetWaitInt 0)
  (return _returnvalue))