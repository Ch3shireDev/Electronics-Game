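; ElectronicsLibrary is a Blueprint function library of shared helpers for HUD access and mouse projection.
; GetElectronicsHUD returns player 0's HUD cast to ElectronicsHUD, or an empty result if the cast fails.
; Project Mouse deprojects the cursor into a world ray and intersects it with the X = 0 plane, mapping the mouse onto a flat YZ working plane.
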(fn GetElectronicsHUD
  (bind _aselectronics_hud (Utilities|Casting|CastToElectronicsHUD (HUD|GetHUD (Game|GetPlayerController (LocalVariables|Get__WorldContext))))
    (:then
      (return _aselectronics_hud))
    (:CastFailed
      (return 0))))

(fn ProjectMouse
  (bind ___worldcontext (LocalVariables|Get__WorldContext))
  (bind _returnvalue (Game|GetPlayerController ___worldcontext))
  (bind (_worldlocation _worlddirection) (Game|Player|ConvertMouseLocationToWorldSpace _returnvalue))
  (if (== (.X (Math|Vector|BreakVector _worldlocation)) 0.0)
    (return _worldlocation)
    (else
      (return (+ _worldlocation (* _worlddirection (- 0.0 (/ (.X (Math|Vector|BreakVector _worldlocation)) (.X (Math|Vector|BreakVector _worlddirection))))))))))